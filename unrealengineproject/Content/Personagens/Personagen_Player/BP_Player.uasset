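; Player character with axe melee, bow shooting, crouch and stamina-limited sprint.
; Light and strong attacks play montage chains, advanced by a `combo` event when input is buffered, with `launch` adding forward lunges.
; FlipFlop keys toggle weapons: the bow pulls in the camera via timelines and spawns arrows along camera rotation, while events swap socketed weapon visibility.
; Sprint macros drain and regenerate stamina through looping timers, alongside a stamina widget created at BeginPlay.
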(event Custom|combo
  ;[1 1 1] combo
  ;;[1 1 1] verificando se o player apertou a tempo de fzr o combo
  (if (Variables|Default|Getsequencia)
    (Variables|Default|Setsequencia false)
    (if (Variables|Default|GetSequip)
      ;;[1 1 1] sistema de combo
      (switch int (Variables|Default|Getint%20Attack)
        (:1
          (Variables|Default|Setint%20Attack 2)
          (Variables|Default|SetAnimmontage "/Game/Personagens/Personagen_Player/comuns/Anim/Machado_equipado/Attack_3.Attack_3")
          ;;;[1 1 1] setando o pulo para frente
          (Variables|Default|SetLaunch%20F 6e+02))
        (:2
          (Variables|Default|Setint%20Attack 3)
          (Variables|Default|SetAnimmontage "/Game/Personagens/Personagen_Player/comuns/Anim/Machado_equipado/Attack_6.Attack_6")
          (Variables|Default|SetLaunch%20F 1.2e+03))
        (:3
          (Variables|Default|SetAnimmontage "/Game/Personagens/Personagen_Player/comuns/Anim/Machado_equipado/Attack_7.Attack_7")
          (Variables|Default|SetLaunch%20F 6e+02))
        (:4
          (Variables|Default|Setint%20Attack 5)
          (Variables|Default|SetAnimmontage "/Game/Personagens/Personagen_Player/comuns/Anim/Machado_equipado/Attack_1.Attack_1")
          (Variables|Default|SetLaunch%20F 1.2e+03))
        (:5
          (Variables|Default|SetAnimmontage "/Game/Personagens/Personagen_Player/comuns/Anim/Machado_equipado/Attack_2.Attack_2")
          (Variables|Default|SetLaunch%20F 6e+02)))
      (Animation|PlayAnimMontage (Variables|Default|GetAnimmontage) 1.0 "None"))))

(event Custom|visableS
  (bind _machadoequipado (Variables|Default|Getmachadoequipado))
  (bind _machado (Variables|Default|Getmachado))
  ;[1 1 1] visibilidade das armas
  (Utilities|FlowControl|FlipFlop
    (:A
      (Rendering|SetVisibility _machadoequipado true false)
      (Rendering|SetVisibility _machado false false))
    (:B
      (Rendering|SetVisibility _machadoequipado false false)
      (Rendering|SetVisibility _machado true false))))

(event Custom|fire
  ;[1 1 1] BOW
  (if (Variables|Default|Getequiped)
    (if (Variables|Default|Getcanshoot)
      (Variables|Default|Setcanshoot false)
      (Animation|StopAnimMontage "/Game/Personagens/Personagen_Player/comuns/Anim/Arco_equipado/draw.draw")
      (Animation|PlayAnimMontage "/Game/Personagens/Personagen_Player/comuns/Anim/Arco_equipado/recoil.recoil" 1.0 "None")
      (Variables|Default|Setshoot true)
      (Audio|PlaySoundatLocation 0 (Transformation|GetActorLocation))
      (Game|SpawnActorfromClass "/Game/weapons/Bow/F_Flecha_Prop_0_1/BP/Arrow.Arrow_C" (Math|Transform|MakeTransform (Transformation|GetSocketLocation (Variables|Character|GetMesh) "arrow") (Transformation|GetWorldRotation (Variables|Default|GetFollowCamera))) "AlwaysSpawn" 0 0)
      (Variables|Default|Setshoot false)
      (Utilities|FlowControl|Delay 0.5)
      (Variables|Default|Setcanshoot true)
      (Variables|Default|SetArrow%20Speed 0.0))))

(event Custom|launch
  ;[1 1 1] boost
  (Variables|/Script/Engine.CharacterMovementComponent|SetGroundFriction (Variables|Character|GetCharacterMovement) 0.0)
  (Character|LaunchCharacter (+ (* (Class|KismetMathLibrary|CreateVectorfromYawPitch (.Yaw (Math|Rotator|BreakRotator (Transformation|GetActorRotation))) (.Y (Math|Vector|BreakVector (Transformation|GetActorForwardVector))) 1.0) (Variables|Default|GetLaunch%20F)) (Transformation|GetActorUpVector)) false false)
  (Utilities|FlowControl|RetriggerableDelay 0.2)
  (Variables|/Script/Engine.CharacterMovementComponent|SetGroundFriction (Variables|Character|GetCharacterMovement) 8.0))

(event Custom|reset
  ;[1 1 1] combo
  ;;[1 1 1] resetando o combo
  (Variables|/Script/Engine.CharacterMovementComponent|SetMaxWalkSpeed (Variables|Character|GetCharacterMovement) 6e+02)
  (Variables|Default|Setsequencia false)
  (Variables|Default|SetAttack false)
  (Variables|Default|Setint%20Attack 1))

(event Custom|visable
  (bind _arcoequipado (Variables|Default|Getarcoequipado))
  (bind _arco (Variables|Default|Getarco))
  ;[1 1 1] visibilidade das armas
  (Utilities|FlowControl|FlipFlop
    (:A
      (Rendering|SetVisibility _arcoequipado true false)
      (Rendering|SetVisibility _arco false false))
    (:B
      (Rendering|SetVisibility _arcoequipado false false)
      (Rendering|SetVisibility _arco true false))))

(event EventBeginPlay
  (bind _returnvalue (UserInterface|CreateWidget "/Game/HUD/stamin.stamin_C"))
  (UserInterface|Viewport|AddtoViewport _returnvalue 0))

(event Input|KeyboardEvents|E
  (params (Key :type Key%20Structure))
  (bind _cameraboom (Variables|Default|GetCameraBoom))
  (bind _charactermovement (Variables|Character|GetCharacterMovement))
  (bind _cameraboom_2 (Variables|Default|GetCameraBoom))
  ;[1 1 1] Equipando o Arco
  (:Pressed
    (Utilities|FlowControl|FlipFlop
      (:A
        (bind _arco (Timeline|Timeline_0 PlayFromStart)
          (:Update
            (Variables|/Script/Engine.SpringArmComponent|SetTargetArmLength _cameraboom (Math|Float|Lerp 3e+02 1.5e+02 _arco))
            (Variables|/Script/Engine.SpringArmComponent|SetSocketOffset _cameraboom (Math|Vector|Lerp(Vector) "0, 0, 0" "0,60.000000, 0" _arco)))
          (:Finished
            (Animation|PlayAnimMontage "/Game/Personagens/Personagen_Player/comuns/Anim/equipe.equipe" 1.0 "None")
            (Variables|Default|Setequiped true)
            (Variables|/Script/Engine.CharacterMovementComponent|SetMaxWalkSpeed _charactermovement 225.0))))
      (:B
        (bind _arco_2 (Timeline|Timeline_1 ReverseFromEnd)
          (:Update
            (Variables|/Script/Engine.SpringArmComponent|SetTargetArmLength _cameraboom_2 (Math|Float|Lerp 3e+02 1.5e+02 _arco_2))
            (Variables|/Script/Engine.SpringArmComponent|SetSocketOffset _cameraboom_2 (Math|Vector|Lerp(Vector) "0, 0, 0" "0,60.000000, 0" _arco_2)))
          (:Finished
            (Animation|PlayAnimMontage "/Game/Personagens/Personagen_Player/comuns/Anim/disarm.disarm" 1.0 "None")
            (Variables|Default|Setequiped false)
            (Variables|/Script/Engine.CharacterMovementComponent|SetMaxWalkSpeed _charactermovement 4.5e+02)))))))

(event Input|MouseEvents|LeftMouseButton
  (params (Key :type Key%20Structure))
  (bind _sequip (Variables|Default|GetSequip))
  ;[1 1 1] combo
  (:Pressed
    ;;[1 1 1] esta com a espada?
    (if _sequip
      (Variables|Default|Setpunching true)
      (Variables|/Script/Engine.CharacterMovementComponent|SetMaxWalkSpeed (Variables|Character|GetCharacterMovement) 0.0)
      (if (Variables|Default|GetAttack)
        (Variables|Default|Setsequencia true)
        (else
          (Variables|Default|SetAttack true)
          (if (Variables|Default|Getstrong)
            (Variables|Default|Setint%20Attack 4)
            (elif (Variables|Default|GetSequip)
              ;;[1 1 1] sistema de combo
              (switch int (Variables|Default|Getint%20Attack)
                (:1
                  (Variables|Default|Setint%20Attack 2)
                  (Variables|Default|SetAnimmontage "/Game/Personagens/Personagen_Player/comuns/Anim/Machado_equipado/Attack_3.Attack_3")
                  ;;;[1 1 1] setando o pulo para frente
                  (Variables|Default|SetLaunch%20F 6e+02))
                (:2
                  (Variables|Default|Setint%20Attack 3)
                  (Variables|Default|SetAnimmontage "/Game/Personagens/Personagen_Player/comuns/Anim/Machado_equipado/Attack_6.Attack_6")
                  (Variables|Default|SetLaunch%20F 1.2e+03))
                (:3
                  (Variables|Default|SetAnimmontage "/Game/Personagens/Personagen_Player/comuns/Anim/Machado_equipado/Attack_7.Attack_7")
                  (Variables|Default|SetLaunch%20F 6e+02))
                (:4
                  (Variables|Default|Setint%20Attack 5)
                  (Variables|Default|SetAnimmontage "/Game/Personagens/Personagen_Player/comuns/Anim/Machado_equipado/Attack_1.Attack_1")
                  (Variables|Default|SetLaunch%20F 1.2e+03))
                (:5
                  (Variables|Default|SetAnimmontage "/Game/Personagens/Personagen_Player/comuns/Anim/Machado_equipado/Attack_2.Attack_2")
                  (Variables|Default|SetLaunch%20F 6e+02)))
              (Animation|PlayAnimMontage (Variables|Default|GetAnimmontage) 1.0 "None")))))))
  (:Released
    (if _sequip
      (Variables|Default|Setpunching false))))

(event Input|MouseEvents|RightMouseButton
  (params (Key :type Key%20Structure))
  (bind _sequip (Variables|Default|GetSequip))
  ;[1 1 1] combo
  (:Pressed
    ;;[1 1 1] esta com a espada?
    (if _sequip
      ;;[1 1 1] Ataque forte
      (Variables|Default|Setstrong true)
      (Variables|Default|Setpunching true)
      (Variables|/Script/Engine.CharacterMovementComponent|SetMaxWalkSpeed (Variables|Character|GetCharacterMovement) 0.0)
      (if (Variables|Default|GetAttack)
        (Variables|Default|Setsequencia true)
        (else
          (Variables|Default|SetAttack true)
          (if (Variables|Default|Getstrong)
            (Variables|Default|Setint%20Attack 4)
            (elif (Variables|Default|GetSequip)
              ;;[1 1 1] sistema de combo
              (switch int (Variables|Default|Getint%20Attack)
                (:1
                  (Variables|Default|Setint%20Attack 2)
                  (Variables|Default|SetAnimmontage "/Game/Personagens/Personagen_Player/comuns/Anim/Machado_equipado/Attack_3.Attack_3")
                  ;;;[1 1 1] setando o pulo para frente
                  (Variables|Default|SetLaunch%20F 6e+02))
                (:2
                  (Variables|Default|Setint%20Attack 3)
                  (Variables|Default|SetAnimmontage "/Game/Personagens/Personagen_Player/comuns/Anim/Machado_equipado/Attack_6.Attack_6")
                  (Variables|Default|SetLaunch%20F 1.2e+03))
                (:3
                  (Variables|Default|SetAnimmontage "/Game/Personagens/Personagen_Player/comuns/Anim/Machado_equipado/Attack_7.Attack_7")
                  (Variables|Default|SetLaunch%20F 6e+02))
                (:4
                  (Variables|Default|Setint%20Attack 5)
                  (Variables|Default|SetAnimmontage "/Game/Personagens/Personagen_Player/comuns/Anim/Machado_equipado/Attack_1.Attack_1")
                  (Variables|Default|SetLaunch%20F 1.2e+03))
                (:5
                  (Variables|Default|SetAnimmontage "/Game/Personagens/Personagen_Player/comuns/Anim/Machado_equipado/Attack_2.Attack_2")
                  (Variables|Default|SetLaunch%20F 6e+02)))
              (Animation|PlayAnimMontage (Variables|Default|GetAnimmontage) 1.0 "None")))))))
  (:Released
    (if _sequip
      (Variables|Default|Setstrong false)
      (Variables|Default|Setpunching false))))

(event Input|KeyboardEvents|Q
  (params (Key :type Key%20Structure))
  (bind _charactermovement (Variables|Character|GetCharacterMovement))
  ;[1 1 1] Desequipando espada
  (:Pressed
    (Utilities|FlowControl|FlipFlop
      (:A
        (Animation|PlayAnimMontage "/Game/Personagens/Personagen_Player/comuns/Anim/WithDrawingS.WithDrawingS" 1.0 "None")
        (Variables|Default|SetSequip true)
        (Variables|/Script/Engine.CharacterMovementComponent|SetMaxWalkSpeed _charactermovement 3e+02))
      (:B
        (Animation|PlayAnimMontage "/Game/Personagens/Personagen_Player/comuns/Anim/sheathingS.sheathingS" 1.0 "None")
        (Variables|Default|SetSequip false)
        (Variables|/Script/Engine.CharacterMovementComponent|SetMaxWalkSpeed _charactermovement 4.5e+02)))))

(event Input|KeyboardEvents|LeftShift
  (params (Key :type Key%20Structure))
  (bind _charactermovement (Variables|Character|GetCharacterMovement))
  ;[1 1 1] stamina
  (:Pressed
    (Components|Timeline|SetPlayRate (Variables|Character|GetMesh) 1.6)
    (|toparado_2
      (:else
        (bind _returnvalue (|decrease_2 _charactermovement (stale _returnvalue_2) 0.05 2.0 0.5 9e+02 4.5e+02)
          (:then
            (goto _label execute3))
          (:then2
            (|final_2 (delegate increase_2) :!label _label))))))
  (:Released
    (Components|Timeline|SetPlayRate (Variables|Character|GetMesh) 1e+01)
    (bind _returnvalue_2 (|increase_2 _charactermovement _returnvalue 0.1 0.18 2.0 0.6 4.5e+02))
    (goto _label execute2)))

(event Input|MouseEvents|LeftMouseButton
  (params (Key :type Key%20Structure))
  ;[1 1 1] BOW
  (:Pressed
    (if (Variables|Default|Getcanshoot)
      (Animation|PlayAnimMontage "/Game/Personagens/Personagen_Player/comuns/Anim/Arco_equipado/draw.draw" 1.0 "None")))
  (:Released
    (if (Variables|Default|Getcanshoot)
      (if (Variables|Default|Getequiped)
        (if (Variables|Default|Getcanshoot)
          (Variables|Default|Setcanshoot false)
          (Animation|StopAnimMontage "/Game/Personagens/Personagen_Player/comuns/Anim/Arco_equipado/draw.draw")
          (Animation|PlayAnimMontage "/Game/Personagens/Personagen_Player/comuns/Anim/Arco_equipado/recoil.recoil" 1.0 "None")
          (Variables|Default|Setshoot true)
          (Audio|PlaySoundatLocation 0 (Transformation|GetActorLocation))
          (Game|SpawnActorfromClass "/Game/weapons/Bow/F_Flecha_Prop_0_1/BP/Arrow.Arrow_C" (Math|Transform|MakeTransform (Transformation|GetSocketLocation (Variables|Character|GetMesh) "arrow") (Transformation|GetWorldRotation (Variables|Default|GetFollowCamera))) "AlwaysSpawn" 0 0)
          (Variables|Default|Setshoot false)
          (Utilities|FlowControl|Delay 0.5)
          (Variables|Default|Setcanshoot true)
          (Variables|Default|SetArrow%20Speed 0.0))))))

(event Input|KeyboardEvents|Tab
  (params (Key :type Key%20Structure))
  ;[1 1 1] crouch
  (:Pressed
    (Utilities|FlowControl|FlipFlop
      (:A
        (Character|Crouch))
      (:B
        (Character|UnCrouch)))))

(fn ConstructionScript
  (Transformation|AttachComponentToComponent (Variables|Default|Getarco) (Variables|Character|GetMesh) "arco" "SnapToTarget" "KeepRelative" "KeepRelative" false)
  (Transformation|AttachComponentToComponent (Variables|Default|Getmachado) (Variables|Character|GetMesh) "machado" "SnapToTarget" "KeepRelative" "KeepRelative" false)
  (Transformation|AttachComponentToComponent (Variables|Default|Getarcoequipado) (Variables|Character|GetMesh) "E_arco" "SnapToTarget" "KeepRelative" "KeepRelative" false)
  (Transformation|AttachComponentToComponent (Variables|Default|Getmachadoequipado) (Variables|Character|GetMesh) "E_machado" "SnapToTarget" "KeepRelative" "KeepRelative" false))

(event Custom|increase%20stamina
  (Utilities|FlowControl|Sequence
    (:then_0
      (bind _output_get (Variables|Default|Setcurrentstaminasprint (+ (Variables|Default|Getcurrentstaminasprint) (stale _tantoqueganha))))
      (if (not (<= _output_get 1e+02))
        (Utilities|Time|ClearandInvalidateTimerbyHandle (stale _returnvalue))
        (return (stale _returnvalue) (delegate Custom|increase%20stamina))))
    (:then_1
      (if (Variables|Default|GetbIsCrouched)
        (Variables|Default|Setcurrentstaminasprint (+ _output_get (stale _agachado)))))))

(event Custom|decrease%20stamina
  (if (AI|Components|NavMovement|IsFalling (Variables|Character|GetCharacterMovement))
    (Variables|Default|Setcurrentstaminasprint (- (Variables|Default|Getstaminaratesprint) (stale _pulando)))
    (else
      (|toparado2_2
        (:then
          (CallFunction|IncreaseStamina))
        (:else
          (bind _output_get (Variables|Default|Setcurrentstaminasprint (- (Variables|Default|Getcurrentstaminasprint) (stale _tantoqueperde))))
          (if (<= _output_get 0.0)
            (Utilities|Time|ClearandInvalidateTimerbyHandle (stale _returnvalue))
            (Variables|/Script/Engine.CharacterMovementComponent|SetMaxWalkSpeed (Variables|Character|GetCharacterMovement) (stale _n_walk))
            (|Outputs (stale _returnvalue)) ; enters at then2
          ))))))